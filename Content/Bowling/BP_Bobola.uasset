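; BP_Bobola is the player-controlled bowling ball, aimed and thrown with the mouse.
; The mouse wheel yaws an Arrow component to set the throw direction.
; Left click, gated by a DoOnce, enables physics on the ball and applies an impulse along the arrow's forward vector, scaled by ThrowSpeed.
; Right click opens the "Gota" level and resets the DoOnce.
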(event `InputAxisKey|MouseWheelAxis`
  (params (AxisValue :type "Float (single-precision)"))
  (`SceneComponent.K2_AddLocalRotation` (`self.Arrow`) (`KismetMathLibrary.MakeRotator` 0.0 0.0 AxisValue) false false))

(event `Key|LeftMouseButton`
  (params (Key :type "Key Structure"))
  (bind _bowlingball (`self.BowlingBall`))
  (:`Pressed`
    (`/Engine/EditorBlueprintResources/StandardMacros.DoOnce` false :!label _label
      (:`Completed`
        (`PrimitiveComponent.SetSimulatePhysics` _bowlingball true)
        (`PrimitiveComponent.AddImpulse` _bowlingball (* (`SceneComponent.GetForwardVector` (`self.Arrow`)) (`self.ThrowSpeed`)) "None" false)))))

(event `Key|RightMouseButton`
  (params (Key :type "Key Structure"))
  (:`Pressed`
    (`GameplayStatics.OpenLevel` "Gota")
    (goto _label :!via `Reset`)))

(fn `UserConstructionScript`)