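; BP_Counter is a bowling score counter that counts pins entering its trigger Box.
; On overlap, it destroys any actor whose class is exactly BP_Pin and increments Score.
; It then updates the ScoreKeeper text by appending the count to a literal "Score: 0" prefix, so a zero always precedes the number.
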(event `self.Box.OnComponentBeginOverlap`
  (params (OverlappedComponent :type "PrimitiveComponent Object Reference") (OtherActor :type "Actor Object Reference") (OtherComp :type "PrimitiveComponent Object Reference") (OtherBodyIndex :type Integer) (bFromSweep :type Boolean) (SweepResult :type "HitResult Structure (by ref)"))
  (if (== (`GameplayStatics.GetObjectClass` OtherActor) "/Game/Bowling/BP_Pin.BP_Pin_C")
    (`self.K2_DestroyActor` OtherActor)
    (bind _result (`/Engine/EditorBlueprintResources/StandardMacros.IncrementInt` (`self.Score`))
      (:`  `
        (`TextRenderComponent.K2_SetText` (`self.ScoreKeeper`) (`KismetTextLibrary.Conv_StringToText` (`KismetStringLibrary.Concat_StrStr` "Score: 0" (`KismetStringLibrary.Conv_IntToString` _result))))))))

(fn `UserConstructionScript`)