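; Player Blueprint with mouse look and a physics-object grab on the left motion controller trigger, with debug prints.
; Pressing line-traces forward from the left controller for physics bodies, intending to disable simulation and attach the actor at HeldObjectLocation.
; The branch after the trace is fixed to false, so pickup never completes as written.
; Releasing detaches any held actor, restores physics and clears the held state.
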(event `InputAction|MotionControllerLeftTrigger`
  (params (Key :type "Key Structure"))
  ;[1 1 1] Holding and Droping of items
  (:`Pressed`
    (if (not (`self.IsHoldingObject`))
      (`self.PickUpObject`)
      (`KismetSystemLibrary.PrintString` "Hello")))
  (:`Released`
    (`self.DropObject`)
    (`KismetSystemLibrary.PrintString` "Bye")))

(event `InputVectorAxis|Mouse2D`
  (params (AxisValue :type "Vector Structure"))
  ;[0 0 0] Mov Camera Mouse
  (`self.AddControllerYawInput` (.x AxisValue))
  (`self.AddControllerPitchInput` (.y AxisValue)))

(event `PickUpObject`
  (bind _mc_left (`self.MC_Left`))
  (bind _hitcomponent (`self.HitComponent`))
  (bind _returnvalue (`SceneComponent.K2_GetComponentLocation` _mc_left))
  ;[0.4062 0.1239 0.3404] PickUp
  (bind _outhit (`KismetSystemLibrary.LineTraceSingleForObjects` :`Start` _returnvalue :`End` (+ _returnvalue (* (`SceneComponent.GetForwardVector` _mc_left) 1000.0)) :`ObjectTypes` (`|MakeArray` "ObjectTypeQuery4" :!type "EObjectTypeQuery Enum") :`DrawDebugType` "ForDuration"))
  (if false
    (bind (_bblockinghit _binitialoverlap _time _distance _location _impactpoint _normal _impactnormal _physmat _hitactor _hitcomponent_2) (`GameplayStatics.BreakHitResult` _outhit))
    (set `self.HitComponent` _hitcomponent_2)
    (if (`SceneComponent.IsAnySimulatingPhysics` _hitcomponent)
      (bind _output_get (set `self.PickedUpActor` _hitactor))
      (`PrimitiveComponent.SetSimulatePhysics` _hitcomponent false)
      (`self.K2_AttachToComponent` _output_get (`self.HeldObjectLocation`) "None" "SnapToTarget" "SnapToTarget" "KeepWorld" true)
      (set `self.IsHoldingObject` true))))

(event `DropObject`
  (bind _pickedupactor (`self.PickedUpActor`))
  (bind _hitcomponent (`self.HitComponent`))
  ;[0.1322 0.3958 0.2961] Drop
  (`/Engine/EditorBlueprintResources/StandardMacros.IsValid` _pickedupactor
    (:`Is Valid`
      (`self.K2_DetachFromActor` _pickedupactor "KeepWorld" "KeepWorld" "KeepWorld")
      (`/Engine/EditorBlueprintResources/StandardMacros.IsValid` _hitcomponent
        (:`Is Valid`
          (`PrimitiveComponent.SetSimulatePhysics` _hitcomponent true)
          (set `self.IsHoldingObject` false)
          (set `self.HitComponent` null)
          (set `self.PickedUpActor` null))))))

(fn `UserConstructionScript`)